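; Gollem enemy that walks toward the player on a 2D plane and performs a jump slam at close range.
; Tick moves it along an X/Z direction refreshed on a delay or hit, with BeginPlay aligning its Y to the player.
; The slam uses flipbook swaps, delays and a cooldown, shaking the camera and randomly damaging players still nearby.
; At zero health it plays death effects once, increments the game instance's WaveKills and destroys itself.
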(event `self.ReceiveBeginPlay`
  (bind (_returnvalue_x _returnvalue_y _returnvalue_z) (`KismetMathLibrary.BreakVector` (`self.K2_GetActorLocation`)))
  (bind (_returnvalue_x_2 _returnvalue_y_2) (`KismetMathLibrary.BreakVector` (`self.K2_GetActorLocation` (`GameplayStatics.GetPlayerPawn` 0))))
  (`self.K2_SetActorLocation` (`KismetMathLibrary.MakeVector` _returnvalue_x (+ _returnvalue_y_2 -1.0) _returnvalue_z) false true))

(event `self.ReceiveHit`
  (params (MyComp :type "PrimitiveComponent Object Reference") (Other :type "Actor Object Reference") (OtherComp :type "PrimitiveComponent Object Reference") (bSelfMoved :type Boolean) (HitLocation :type "Vector Structure") (HitNormal :type "Vector Structure") (NormalImpulse :type "Vector Structure") (Hit :type "HitResult Structure (by ref)"))
  (set `self.CanSet` true))

(event `self.ReceiveTick`
  (params (DeltaSeconds :type "Float (single-precision)"))
  (bind (_returnvalue_x _returnvalue_y _returnvalue_z) (`KismetMathLibrary.BreakVector` (`self.K2_GetActorLocation`)))
  (bind _asplayer_bp (cast `/Game/Player/PlayerBP` (`GameplayStatics.GetPlayerPawn` 0) :!pure true))
  (bind _asccgame_instance (cast `/Game/Engine/CCGameInstance` (`GameplayStatics.GetGameInstance`) :!pure true))
  (bind (_returnvalue_x_2 _returnvalue_y_2 _returnvalue_z_2) (`KismetMathLibrary.BreakVector` (`KismetMathLibrary.GetForwardVector` (`KismetMathLibrary.FindLookAtRotation` (`self.K2_GetActorLocation`) (`self.K2_GetActorLocation` (`GameplayStatics.GetPlayerPawn` 0))))))
  (if (> (`self.Health`) 0)
    (if (not (`self.IsJumping?`))
      (`self.AddMovementInput` (`self.PlayerDir`) 10.0))
    (if (`self.CanSet`)
      (set `self.CanSet` false)
      (set `self.PlayerDir` (`KismetMathLibrary.MakeVector` _returnvalue_x_2 0.0 _returnvalue_z_2))
      (`KismetSystemLibrary.Delay` 3.0)
      (set `self.CanSet` true)
      (elif (`self.IsJumping?`)
        _
        (elif (<= (`self.GetDistanceTo` (`GameplayStatics.GetPlayerPawn` 0)) 100.0)
          (if (== (`self.JumpCool`) 0.0)
            (set `self.JumpCool` 5.0)
            (`PaperFlipbookComponent.SetFlipbook` (`self.Sprite`) "/Game/Enemy/Gollem/Jump_FB.Jump_FB")
            (bind _returnvalue (`AddComponent|NODE_AddAudioComponent-1` :`RelativeTransform` (`self.GetTransform`)))
            (set `self.IsJumping?` true)
            (`KismetSystemLibrary.Delay` 0.7)
            (if (> (`self.Health`) 0)
              (`GameplayStatics.SpawnEmitterAtLocation` "/Game/Effects/ParticleEffects/Smoke/Dust.Dust" (`KismetMathLibrary.MakeVector` _returnvalue_x _returnvalue_y (- _returnvalue_z 10.0)))
              (`PlayerController.ClientStartCameraShake` :`self` (`GameplayStatics.GetPlayerController` 0) :`Shake` "/Game/Shakes/HeavyShake.HeavyShake_C")
              (if (<= (`self.GetDistanceTo` (`GameplayStatics.GetPlayerPawn` 0)) 100.0)
                (set `/Game/Player/PlayerBP.Health` (- (`/Game/Player/PlayerBP.Health` _asplayer_bp) (`KismetMathLibrary.RandomIntegerInRange` 10 25)) _asplayer_bp))
              (`KismetSystemLibrary.Delay` 0.2)
              (set `self.IsJumping?` false)
              (`PaperFlipbookComponent.SetFlipbook` (`self.Sprite`) "/Game/Enemy/Gollem/Gollem_FB.Gollem_FB"))
            (else
              (set `self.JumpCool` (`KismetMathLibrary.FInterpTo_Constant` (`self.JumpCool`) 0.0 (`GameplayStatics.GetWorldDeltaSeconds`) 1.0) :!label _label)))
          (else
            (goto _label)))))
    (else
      (`/Engine/EditorBlueprintResources/StandardMacros.DoOnce` false
        (:`Completed`
          (`AudioComponent.Stop` _returnvalue)
          (`GameplayStatics.PlaySound2D` "/Game/Sound/EnemyKill.EnemyKill" 1.0 1.0 0.0 null null)
          (`GameplayStatics.SpawnEmitterAtLocation` "/Game/Effects/ParticleEffects/Smoke/Smoke_Part.Smoke_Part" (`self.K2_GetActorLocation`))
          (`SceneComponent.SetVisibility` (`self.Sprite`) false false)
          (set `/Game/Engine/CCGameInstance.WaveKills` (+ (`/Game/Engine/CCGameInstance.WaveKills` _asccgame_instance) 1) _asccgame_instance)
          (`KismetSystemLibrary.Delay` 1.0)
          (`self.K2_DestroyActor`))))))

(fn `UserConstructionScript`)