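; Mage enemy for a 2D sprite game that keeps its distance from the player while casting fireballs.
; Each Tick it moves along the X/Z direction to the player, retreating when close and approaching otherwise.
; Tick also calls the fireball event before the health check, with a Delay spacing spawns about two seconds apart.
; At zero health it plays death effects once, credits coins and a wave kill to CCGameInstance, then destroys itself.
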(event `self.ReceiveTick`
  (params (DeltaSeconds :type "Float (single-precision)"))
  (bind _playerforwardvector (`self.PlayerForwardVector`))
  (bind _returnvalue (<= (`self.GetDistanceTo` (`GameplayStatics.GetPlayerPawn` 0)) 200.0))
  (bind (_returnvalue_x _returnvalue_y _returnvalue_z) (`KismetMathLibrary.BreakVector` (`KismetMathLibrary.GetForwardVector` (`KismetMathLibrary.FindLookAtRotation` (`self.K2_GetActorLocation`) (`self.K2_GetActorLocation` (`GameplayStatics.GetPlayerPawn` 0))))))
  (`self.FIREABAL`)
  (if (> (`self.Health`) 0)
    (set `self.PlayerForwardVector` (`KismetMathLibrary.MakeVector` _returnvalue_x 0.0 _returnvalue_z))
    (if _returnvalue
      (`self.AddMovementInput` _playerforwardvector -1.0)
      (else
        (`self.AddMovementInput` _playerforwardvector 0.7)))
    (if _returnvalue
      _)
    (else
      (`/Engine/EditorBlueprintResources/StandardMacros.DoOnce` false
        (:`Completed`
          (`GameplayStatics.PlaySound2D` "/Game/Sound/EnemyKill.EnemyKill" 1.0 1.0 0.0 null null)
          (`GameplayStatics.SpawnEmitterAtLocation` "/Game/Effects/ParticleEffects/Smoke/Smoke_Part.Smoke_Part" (`self.K2_GetActorLocation`))
          (`SceneComponent.SetVisibility` (`self.Sprite`) false false)
          (bind _asccgame_instance (cast `/Game/Engine/CCGameInstance` (`GameplayStatics.GetGameInstance`)))
          (set `/Game/Engine/CCGameInstance.Coins` (+ (`/Game/Engine/CCGameInstance.Coins` _asccgame_instance) 10) _asccgame_instance)
          (set `/Game/Engine/CCGameInstance.WaveKills` (+ (`/Game/Engine/CCGameInstance.WaveKills` _asccgame_instance) 1) _asccgame_instance)
          (`KismetSystemLibrary.Delay` 1.0)
          (`self.K2_DestroyActor`))))))

(event `FIREABAL`
  (`KismetSystemLibrary.Delay` 2.0)
  (`|SpawnActorFromClass` "/Game/Enemy/Mage/Fireball_BP.Fireball_BP_C" (`KismetMathLibrary.Conv_VectorToTransform` (`self.K2_GetActorLocation`)) "Undefined" "OverrideRootScale" null null))

(fn `UserConstructionScript`)