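; Fireball projectile for the Mage enemy that launches at the player and deals damage on contact.
; On BeginPlay it snaps its Y to the player pawn's Y, keeping motion on the player's plane, then aims a constant-speed ProjectileMovement velocity at the player's current position without homing.
; Overlapping a PlayerBP subtracts Health directly, plays a camera shake and hit sound, then destroys the fireball.
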(event `self.ReceiveActorBeginOverlap`
  (params (OtherActor :type "Actor Object Reference"))
  (bind _asplayer_bp (cast `/Game/Player/PlayerBP` OtherActor))
  (set `/Game/Player/PlayerBP.Health` (- (`/Game/Player/PlayerBP.Health` _asplayer_bp) 10) _asplayer_bp)
  (`PlayerController.ClientStartCameraShake` :`self` (`GameplayStatics.GetPlayerController` 0) :`Shake` "/Game/Shakes/SlightShake.SlightShake_C")
  (`GameplayStatics.PlaySound2D` "/Game/Sound/Hit.Hit" 1.0 1.0 0.0 null null)
  (`self.K2_DestroyActor`))

(event `self.ReceiveBeginPlay`
  (bind (_returnvalue_x _returnvalue_y _returnvalue_z) (`KismetMathLibrary.BreakVector` (`self.K2_GetActorLocation`)))
  (bind _returnvalue (`GameplayStatics.GetPlayerPawn` 0))
  (bind (_returnvalue_x_2 _returnvalue_y_2) (`KismetMathLibrary.BreakVector` (`self.K2_GetActorLocation` _returnvalue)))
  (`self.K2_SetActorLocation` (`KismetMathLibrary.MakeVector` _returnvalue_x _returnvalue_y_2 _returnvalue_z))
  (set `MovementComponent.Velocity` (* (`KismetMathLibrary.GetForwardVector` (`KismetMathLibrary.FindLookAtRotation` (`self.K2_GetActorLocation`) (`self.K2_GetActorLocation` _returnvalue))) 250.0) (`self.ProjectileMovement`)))

(fn `UserConstructionScript`)