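; Scavenger enemy with a sprite that charges the player and deals random contact damage, unless the player is lunging or attacking.
; On spawn it snaps to the player's Y, counts itself in CCGameInstance and caches a heading toward the player, re-aimed only on Hit.
; Tick follows that heading until Health runs out, then once plays death effects, awards coins and kill stats, and destroys the actor after a delay.
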(event `self.ReceiveBeginPlay`
  (bind (_returnvalue_x _returnvalue_y _returnvalue_z) (`KismetMathLibrary.BreakVector` (`self.K2_GetActorLocation`)))
  (bind (_returnvalue_x_2 _returnvalue_y_2) (`KismetMathLibrary.BreakVector` (`self.K2_GetActorLocation` (`GameplayStatics.GetPlayerPawn` 0))))
  (`self.K2_SetActorLocation` (`KismetMathLibrary.MakeVector` _returnvalue_x _returnvalue_y_2 _returnvalue_z) false true)
  (set `self.PlayerForwardVector` (* (`KismetMathLibrary.GetForwardVector` (`KismetMathLibrary.FindLookAtRotation` (`self.K2_GetActorLocation`) (`self.K2_GetActorLocation` (`GameplayStatics.GetPlayerPawn` 0)))) 5))
  (bind _asccgame_instance (cast `/Game/Engine/CCGameInstance` (`GameplayStatics.GetGameInstance`)))
  (set `/Game/Engine/CCGameInstance.EnemySpawns` (+ (`/Game/Engine/CCGameInstance.EnemySpawns` _asccgame_instance) 1) _asccgame_instance))

(event `self.ReceiveHit`
  (params (MyComp :type "PrimitiveComponent Object Reference") (Other :type "Actor Object Reference") (OtherComp :type "PrimitiveComponent Object Reference") (bSelfMoved :type Boolean) (HitLocation :type "Vector Structure") (HitNormal :type "Vector Structure") (NormalImpulse :type "Vector Structure") (Hit :type "HitResult Structure (by ref)"))
  (bind (_returnvalue_x _returnvalue_y _returnvalue_z) (`KismetMathLibrary.BreakVector` (`KismetMathLibrary.GetForwardVector` (`KismetMathLibrary.FindLookAtRotation` (`self.K2_GetActorLocation`) (`self.K2_GetActorLocation` (`GameplayStatics.GetPlayerPawn` 0))))))
  (set `self.PlayerForwardVector` (`KismetMathLibrary.MakeVector` _returnvalue_x 0.0 _returnvalue_z)))

(event `self.ReceiveActorBeginOverlap`
  (params (OtherActor :type "Actor Object Reference"))
  (if (> (`self.Health`) 0)
    (bind _asplayer_bp (cast `/Game/Player/PlayerBP` OtherActor))
    (if (> (`/Game/Player/PlayerBP.Health` _asplayer_bp) 0)
      (if (`/Game/Player/PlayerBP.Lunging` _asplayer_bp)
        _
        (elif (not (`/Game/Player/PlayerBP.Attacking` _asplayer_bp))
          (set `/Game/Player/PlayerBP.Health` (- (`/Game/Player/PlayerBP.Health` _asplayer_bp) (`KismetMathLibrary.RandomIntegerInRange` 1 3)) _asplayer_bp)
          (`PlayerController.ClientStartCameraShake` :`self` (`GameplayStatics.GetPlayerController` 0) :`Shake` "/Game/Shakes/SlightShake.SlightShake_C")
          (`GameplayStatics.PlaySound2D` "/Game/Sound/Hit.Hit" 1.0 1.0 0.0 null null))))))

(event `self.ReceiveTick`
  (params (DeltaSeconds :type "Float (single-precision)"))
  (if (> (`self.Health`) 0)
    (`self.AddMovementInput` (`self.PlayerForwardVector`))
    (else
      (`/Engine/EditorBlueprintResources/StandardMacros.DoOnce` false
        (:`Completed`
          (`GameplayStatics.PlaySound2D` "/Game/Sound/EnemyKill.EnemyKill" 1.0 1.0 0.0 null null)
          (`GameplayStatics.SpawnEmitterAtLocation` "/Game/Effects/ParticleEffects/Smoke/Smoke_Part.Smoke_Part" (`self.K2_GetActorLocation`))
          (`SceneComponent.SetVisibility` (`self.Sprite`) false false)
          (bind _asccgame_instance (cast `/Game/Engine/CCGameInstance` (`GameplayStatics.GetGameInstance`)))
          (set `/Game/Engine/CCGameInstance.Coins` (+ (`/Game/Engine/CCGameInstance.Coins` _asccgame_instance) 2) _asccgame_instance)
          (set `/Game/Engine/CCGameInstance.TotalCoins` (+ (`/Game/Engine/CCGameInstance.TotalCoins` _asccgame_instance) 2) _asccgame_instance)
          (set `/Game/Engine/CCGameInstance.WaveKills` (+ (`/Game/Engine/CCGameInstance.WaveKills` _asccgame_instance) 1) _asccgame_instance)
          (set `/Game/Engine/CCGameInstance.TotalEnemyKills` (+ (`/Game/Engine/CCGameInstance.TotalEnemyKills` _asccgame_instance) 1) _asccgame_instance)
          (`KismetSystemLibrary.Delay` 1.0)
          (`self.K2_DestroyActor`))))))

(fn `UserConstructionScript`
  (`parent.UserConstructionScript`))